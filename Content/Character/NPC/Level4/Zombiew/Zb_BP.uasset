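; Zombie NPC for Level 4 that explodes on contact with the player character (Tim_BP), damaging the player and dying.
; A capsule overlap spawns an explosion at the player pawn, zeroes the zombie's Health and subtracts from CharacterHealth stored in Midterm_GI, the game instance.
; It then plays a one-shot dying animation and destroys itself after a short delay, with no guard against repeat overlaps meanwhile.
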(event OnComponentBeginOverlap(Capsule)
  (params (OverlappedComponent :type Primitive%20Component%20Object%20Reference) (OtherActor :type Actor%20Object%20Reference) (OtherComp :type Primitive%20Component%20Object%20Reference) (OtherBodyIndex :type Integer) (bFromSweep :type Boolean) (SweepResult :type Hit%20Result%20Structure%20%28by%20ref%29))
  (Utilities|Casting|CastToTim_BP OtherActor)
  (Effects|SpawnEmitteratLocation "/Game/StarterContent/Particles/P_Explosion.P_Explosion" (Transformation|GetActorLocation (Game|Player|GetPlayerPawn 0)) "0, 0, 0" "2.000000,2.000000,2.000000")
  (Variables|Default|Sethealth 0)
  (bind _asmidterm_gi (Utilities|Casting|CastToMidterm_GI (Game|GetGameInstance)))
  (Variables|/Game/Character/Tim/Midterm_GI.Midterm_GI_C|SetCharacter_Health _asmidterm_gi (- (Variables|/Game/Character/Tim/Midterm_GI.Midterm_GI_C|GetCharacter_Health _asmidterm_gi) 2))
  (Components|Animation|PlayAnimation (Variables|Character|GetMesh) "/Game/Character/NPC/Level4/Zombiew/Animation/zombie_dying.zombie_dying" false)
  (Utilities|FlowControl|Delay 5.0)
  (Actor|DestroyActor))

(fn ConstructionScript)