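; Game mode that respawns the Tim_BP player character after it is destroyed.
; On BeginPlay it binds to the player character's destroyed event.
; After a short delay, that event spawns a new Tim_BP at the SpawnTransform variable, has the player controller possess it and resets CharacterHealth in Midterm_GI.
; It then calls Respawn to rebind on the new pawn, so the cycle repeats.
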(event Custom|DestoryedEvent
  (params (DestroyedActor :type Actor%20Object%20Reference))
  ;[1 1 1] Respawn and check
  (Utilities|FlowControl|Delay 2.0)
  (bind _returnvalue (Game|SpawnActorfromClass "/Game/Character/Tim/Tim_BP.Tim_BP_C" (Variables|Default|GetSpawn%20Transform) "Undefined" 0 0))
  (Pawn|Possess (Game|GetPlayerController 0) _returnvalue)
  (bind _asmidterm_gi (Utilities|Casting|CastToMidterm_GI (Game|GetGameInstance)))
  (Variables|/Game/Character/Tim/Midterm_GI.Midterm_GI_C|SetCharacter_Health _asmidterm_gi 20)
  (CallFunction|Respawn))

(event Custom|Respawn
  ;[1 1 1] Respawn and check
  (bind _astim_bp (Utilities|Casting|CastToTim_BP (Game|GetPlayerCharacter 0)))
  (Game|BindEventtoOnDestroyed _astim_bp (delegate Custom|DestoryedEvent)))

(event EventBeginPlay
  ;[1 1 1] Respawn and check
  (bind _astim_bp (Utilities|Casting|CastToTim_BP (Game|GetPlayerCharacter 0)))
  (Game|BindEventtoOnDestroyed _astim_bp (delegate Custom|DestoryedEvent)))

(fn ConstructionScript)