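; BP_Finish is the Level 4 exit trigger that ends the game when the Tim_BP character arrives holding three keys.
; Overlapping its box turns on a rect light, then quits the game if IsThreeKeys is set, or shows a text render otherwise.
; Leaving the box hides both the text and the light.
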(event OnComponentBeginOverlap(Box)
  (params (OverlappedComponent :type Primitive%20Component%20Object%20Reference) (OtherActor :type Actor%20Object%20Reference) (OtherComp :type Primitive%20Component%20Object%20Reference) (OtherBodyIndex :type Integer) (bFromSweep :type Boolean) (SweepResult :type Hit%20Result%20Structure%20%28by%20ref%29))
  (bind _astim_bp (Utilities|Casting|CastToTim_BP OtherActor))
  (Rendering|SetVisibility (Variables|Default|GetRectLight) true false)
  (if (Variables|/Game/Character/Tim/Tim_BP.Tim_BP_C|GetIsThreeKeys _astim_bp)
    (Game|QuitGame 0 "Quit" false)
    (else
      (Rendering|SetVisibility (Variables|Default|GetTextRender) true false))))

(event OnComponentEndOverlap(Box)
  (params (OverlappedComponent :type Primitive%20Component%20Object%20Reference) (OtherActor :type Actor%20Object%20Reference) (OtherComp :type Primitive%20Component%20Object%20Reference) (OtherBodyIndex :type Integer))
  (Utilities|Casting|CastToTim_BP OtherActor)
  (Rendering|SetVisibility (Variables|Default|GetTextRender) false false)
  (Rendering|SetVisibility (Variables|Default|GetRectLight) false false))

(fn ConstructionScript)