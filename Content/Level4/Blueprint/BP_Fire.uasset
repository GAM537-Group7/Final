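; BP_Fire is a fire hazard that damages the Tim_BP player while inside its capsule.
; Entering spawns a tall fire emitter at the static mesh's relative location and starts a looping one-second timer.
; Each tick subtracts health from the Midterm_GI game instance and calls Death on the player character.
; Leaving pauses the timer and deactivates the emitter.
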(event OnComponentBeginOverlap(Capsule)
  (params (OverlappedComponent :type Primitive%20Component%20Object%20Reference) (OtherActor :type Actor%20Object%20Reference) (OtherComp :type Primitive%20Component%20Object%20Reference) (OtherBodyIndex :type Integer) (bFromSweep :type Boolean) (SweepResult :type Hit%20Result%20Structure%20%28by%20ref%29))
  (Utilities|Casting|CastToTim_BP OtherActor)
  (Utilities|Casting|CastToMidterm_GI (Game|GetGameInstance))
  (bind _returnvalue (Effects|SpawnEmitteratLocation "/Game/StarterContent/Particles/P_Fire.P_Fire" (Variables|/Script/Engine.SceneComponent|GetRelativeLocation (Variables|Debug|GetStaticMeshComponent)) "0, 0, 0" "3.000000,3.000000,15.000000"))
  (Utilities|Time|SetTimerbyFunctionName 0 (Utilities|String|MakeLiteralString "FireDamage") 1.0 true))

(event OnComponentEndOverlap(Capsule)
  (params (OverlappedComponent :type Primitive%20Component%20Object%20Reference) (OtherActor :type Actor%20Object%20Reference) (OtherComp :type Primitive%20Component%20Object%20Reference) (OtherBodyIndex :type Integer))
  (Utilities|Casting|CastToTim_BP OtherActor)
  (Utilities|Casting|CastToMidterm_GI (Game|GetGameInstance))
  (Class|KismetSystemLibrary|PauseTimer 0 (Utilities|String|MakeLiteralString "FireDamage"))
  (Components|Activation|Deactivate (stale OnComponentBeginOverlap(Capsule) _returnvalue)))

(fn ConstructionScript)

(fn FireDamage
  (bind _astim_bp (Utilities|Casting|CastToTim_BP (Game|GetPlayerCharacter 0)))
  (bind _asmidterm_gi (Utilities|Casting|CastToMidterm_GI (Game|GetGameInstance)))
  (Variables|/Game/Character/Tim/Midterm_GI.Midterm_GI_C|SetCharacter_Health _asmidterm_gi (- (Variables|/Game/Character/Tim/Midterm_GI.Midterm_GI_C|GetCharacter_Health _asmidterm_gi) 2))
  (Default|Death _astim_bp))