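; BP_Pass is a Level 4 actor that destroys itself when Tim_BP hits its capsule.
; The hit handler also requires the game instance to be Midterm_GI, but changes nothing on it.
; A separate Explosion function lowers CharacterHealth on the game instance and calls Death on the player's Tim_BP.
; Nothing in this Blueprint calls Explosion, so the hit itself deals no damage.
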(event OnComponentHit(Capsule)
  (params (HitComponent :type Primitive%20Component%20Object%20Reference) (OtherActor :type Actor%20Object%20Reference) (OtherComp :type Primitive%20Component%20Object%20Reference) (NormalImpulse :type Vector :default "0, 0, 0") (Hit :type Hit%20Result%20Structure%20%28by%20ref%29))
  (Utilities|Casting|CastToTim_BP OtherActor)
  (Utilities|Casting|CastToMidterm_GI (Game|GetGameInstance))
  (Actor|DestroyActor))

(fn ConstructionScript)

(fn Explosion
  (bind _astim_bp (Utilities|Casting|CastToTim_BP (Game|GetPlayerCharacter 0)))
  (bind _asmidterm_gi (Utilities|Casting|CastToMidterm_GI (Game|GetGameInstance)))
  (Variables|/Game/Character/Tim/Midterm_GI.Midterm_GI_C|SetCharacter_Health _asmidterm_gi (- (Variables|/Game/Character/Tim/Midterm_GI.Midterm_GI_C|GetCharacter_Health _asmidterm_gi) 5))
  (Default|Death _astim_bp))